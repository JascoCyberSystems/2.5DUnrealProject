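; Player-controlled 2D side-scrolling character that runs, jumps, shoots, climbs and takes damage, with a health HUD created on BeginPlay.
; Input, landing and damage events set CurrentState, which UpdateAnimation maps to sprite flipbooks every tick.
; Tick also turns the character through control rotation based on horizontal velocity and last input direction.
; Non-fatal hits apply knockback and timer-driven flashing invulnerability; X triggers test damage.
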(event `UpdateAnimation`
  ;[1 1 1] Handle Animation
  (switch `/Game/CustomFiles/Blueprints/8BitGuy_States` (`self.currentState`)
    (:`NewEnumerator0`
      (`PaperFlipbookComponent.SetFlipbook` (`self.Sprite`) (select `bool` (> (`KismetMathLibrary.VSize` (`self.GetVelocity`)) 0.0) :`false` "/Game/CustomFiles/Sprites/8BitGuy/8bitA_Idle.8bitA_Idle" :`true` "/Game/CustomFiles/Sprites/8BitGuy/8bitA_Run.8bitA_Run" :!type "PaperFlipbook Object Reference")))
    (:`NewEnumerator12`
      (`PaperFlipbookComponent.SetFlipbook` (`self.Sprite`) null))
    (:`NewEnumerator8`
      (`PaperFlipbookComponent.SetFlipbook` (`self.Sprite`) "/Game/CustomFiles/Sprites/8BitGuy/8bitA_Shoot.8bitA_Shoot"))
    (:`NewEnumerator2`
      (`PaperFlipbookComponent.SetFlipbook` (`self.Sprite`) "/Game/CustomFiles/Sprites/8BitGuy/8bitA_Jumping.8bitA_Jumping"))
    (:`NewEnumerator20`
      (`PaperFlipbookComponent.SetFlipbook` (`self.Sprite`) "/Game/CustomFiles/Sprites/8BitGuy/8bitA_Drop.8bitA_Drop"))
    (:`NewEnumerator18`
      (`PaperFlipbookComponent.SetFlipbook` (`self.Sprite`) "/Game/CustomFiles/Sprites/8BitGuy/8bitA_ClimbGrab.8bitA_ClimbGrab"))
    (:`NewEnumerator7`
      (`PaperFlipbookComponent.SetFlipbook` (`self.Sprite`) "/Game/CustomFiles/Sprites/8BitGuy/8bitA_Climb.8bitA_Climb"))
    (:`NewEnumerator17`
      (`PaperFlipbookComponent.SetFlipbook` (`self.Sprite`) "/Game/CustomFiles/Sprites/8BitGuy/8bitA_Fall.8bitA_Fall"))
    (:`NewEnumerator4`
      (`PaperFlipbookComponent.SetFlipbook` (`self.Sprite`) "/Game/CustomFiles/Sprites/8BitGuy/8bitA_Hit.8bitA_Hit"))
    (:`NewEnumerator5`
      (`PaperFlipbookComponent.SetFlipbook` (`self.Sprite`) "/Game/CustomFiles/Sprites/8BitGuy/8bitA_Die.8bitA_Die"))))

(event `self.ReceiveBeginPlay`
  ;[0 1 0.0615] Initilize
  (`|ExecutionSequence`
    (:`then_0`
      (`ActorComponent.SetIsReplicated` (`self.Sprite`) true))
    (:`then_1`
      (bind _returnvalue (`|CreateWidget` "/Game/CustomFiles/Blueprints/8BitGuy_HUD.8BitGuy_HUD_C" (`GameplayStatics.GetPlayerController` 0)))
      (bind _output_get (set `self.HealthBar` _returnvalue))
      (`UserWidget.AddToViewport` _output_get 0))))

(event `Key|X`
  (params (Key :type "Key Structure"))
  ;[1 0 0.04404] Damage System
  (:`Pressed`
    (`self.PlayerDamage` 0.05)))

(event `PlayerDamage`
  (params (DamageTaken :type "Float (double-precision)"))
  (bind _knockback (`self.knockBack`))
  ;[1 0 0.04404] Damage System
  (if (not (`self.isInvulnerable`))
    (set `self.isHit` true)
    (set `self.hasFallDown` true)
    (`self.DisableInput` (`GameplayStatics.GetPlayerController` 0))
    (bind _output_get (set `self.Current_Health` (- (`self.Current_Health`) DamageTaken)))
    (if (<= _output_get 0.01)
      (set `self.currentState` "NewEnumerator5")
      (`self.UpdateAnimation`)
      (`self.DisableInput` (`GameplayStatics.GetPlayerController` 0))
      (else
        (set `self.currentState` "NewEnumerator4")
        (`self.UpdateAnimation`)
        (`CharacterMovementComponent.AddForce` (`self.CharacterMovement`) (`KismetMathLibrary.MakeVector` (* (`self.Current_Direction`) (* -1.0 _knockback)) 0.0 (* _knockback 2.0)))
        (`KismetSystemLibrary.K2_SetTimer` null "InvulnerabilityFlashing" 0.1 true) ; Enable Invulnerability Flashing
        (set `self.isInvulnerable` true)
        (`KismetSystemLibrary.Delay` 2.0)
        (`KismetSystemLibrary.K2_ClearTimer` null "InvulnerabilityFlashing") ; Disable Invulnerability Flashing
        (set `self.isHit` false)
        (set `self.isInvulnerable` false)
        (`SceneComponent.SetHiddenInGame` (`self.Sprite`) false false :!label _label)))))

(event `InvulnerabilityFlashing`
  ;[1 0 0.04404] Damage System
  (`SceneComponent.SetHiddenInGame` (`self.Sprite`) true false)
  (`KismetSystemLibrary.Delay` 0.05)
  (goto _label))

(event `self.ReceiveTick`
  (params (DeltaSeconds :type "Float (single-precision)"))
  ;[1 1 1] Tick - Updates animation
  (`self.UpdateAnimation`)
  (if (`self.canMove`)
    (if (not (`self.hasFallDown`))
      (`/Engine/EditorBlueprintResources/StandardMacros.CompareFloat` (.x (`MovementComponent.Velocity` (`self.GetMovementComponent`)))
        (:`>`
          (`Controller.SetControlRotation` (`self.GetController`) (`KismetMathLibrary.MakeRotator` 0.0) :!label _label_2)
          (set `self.Current_Direction` 1))
        (:`==`
          (if (`self.isMovingRight`)
            (goto _label_2)
            (else
              (`Controller.SetControlRotation` (`self.GetController`) (`KismetMathLibrary.MakeRotator` 0.0 0.0 180.0) :!label _label_3)
              (set `self.Current_Direction` -1))))
        (:`<`
          (goto _label_3))))))

(event `InputAction|Shoot`
  (params (Key :type "Key Structure"))
  ;[1 1 1] Shooting
  (:`Pressed`
    (if (`self.canShoot`)
      (`MovementComponent.StopMovementImmediately` (`self.CharacterMovement`))
      (set `self.canShoot` false)
      (set `self.canMove` false)
      (`|SpawnActorFromClass` "/Game/CustomFiles/Blueprints/BP_Bullet.BP_Bullet_C" (`SceneComponent.K2_GetComponentToWorld` (`self.ShotDirection`)) "AlwaysSpawn" "OverrideRootScale" null null)
      (set `self.currentState` "NewEnumerator8")
      (`self.UpdateAnimation`)
      (`KismetSystemLibrary.RetriggerableDelay` 0.4 :!label _label_4)
      (set `self.currentState` "NewEnumerator0")
      (set `self.canShoot` true)
      (set `self.canMove` true)
      (`self.UpdateAnimation`)))
  (:`Released`
    (goto _label_4)))

(event `InputAxis|MoveRight`
  (params (AxisValue :type "Float (single-precision)"))
  ;[1 1 1] Handle movement
  (if (`self.canMove`)
    (if (> AxisValue 0.0)
      (set `self.isMovingRight` true)
      (elif (< AxisValue 0.0)
        (set `self.isMovingRight` false)))
    (`self.AddMovementInput` (1.0 0.0 0.0) AxisValue)))

(event `InputAction|Jump`
  (params (Key :type "Key Structure"))
  ;[1 1 1] Jumping/Falling
  (:`Pressed`
    (`self.Jump` :!label _label_5)
    (set `self.currentState` "NewEnumerator2")
    (`self.UpdateAnimation`))
  (:`Released`
    (`self.StopJumping` :!label _label_6)))

(event `InputTouch`
  (params (Location :type "Vector Structure") (FingerIndex :type "ETouchIndex Enum"))
  ;[1 1 1] Jumping/Falling
  (:`Pressed`
    (goto _label_5))
  (:`Released`
    (goto _label_6)))

(event `self.OnLanded`
  (params (Hit :type "HitResult Structure (by ref)"))
  ;[1 1 1] Jumping/Falling
  (if (`self.hasFallDown`)
    (if (not (`self.isHit`))
      (`self.DisableInput` (`GameplayStatics.GetPlayerController` 0)))
    (set `self.canMove` false)
    (set `self.currentState` "NewEnumerator17")
    (`self.UpdateAnimation`)
    (`KismetSystemLibrary.Delay` 0.2)
    (set `self.canMove` true)
    (set `self.hasFallDown` false)
    (`self.EnableInput` (`GameplayStatics.GetPlayerController` 0)))
  (set `self.currentState` "NewEnumerator0")
  (`self.UpdateAnimation`))

(event `InputAction|Grab`
  (params (Key :type "Key Structure"))
  ;[1 1 1] Grab/Climb/Lift
  (:`Pressed`
    (set `self.isGrabbing` true)
    (if (`self.canClimb`)
      (set `self.currentState` "NewEnumerator18")
      (`self.UpdateAnimation` :!label _label_7)))
  (:`Released`
    (set `self.isGrabbing` false)
    (set `self.currentState` "NewEnumerator20" :!label _label_8)
    (goto _label_7)))

(event `InputAxis|MoveUp`
  (params (AxisValue :type "Float (single-precision)"))
  ;[1 1 1] Grab/Climb/Lift
  (if (`self.isGrabbing`)
    (if (`self.canClimb`)
      (set `self.currentState` "NewEnumerator7")
      (`self.UpdateAnimation`)
      (if (>= AxisValue 0.1)
        (`self.K2_AddActorLocalOffset` (`KismetMathLibrary.MakeVector` 0.0 0.0 (* AxisValue (`self.climbSpeed`)))))
      (else
        (goto _label_8)))
    (else
      (goto _label_8))))

(fn `UserConstructionScript`)